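; Actor component running a heartbeat quick-time event where the player presses randomly chosen keys in time with beats.
; StartQTE resets counters and shows the widget; each TriggerHeartbeat picks a random key and timing window.
; Tick compares presses against the target time, counting successes or failures with widget feedback.
; Reaching the success goal starts the character's dialogue-choice QTE, the fail goal plays a level sequence, and both end this QTE.
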(event `Outcome`
  (if (>= (`self.SuccessCount`) (`self.SuccessGoal`))
    (`WidgetBlueprintLibrary.SetInputMode_GameOnly` (`GameplayStatics.GetPlayerController` 0))
    (`/Game/Dynamic/Systems/QTE/Dialogue/BPC_DialogueChoice.Start QTE` (`/Game/Dynamic/ThirdPerson/Blueprints/BP_ThirdPersonCharacter.BPC_DialogueChoice` (`self.As BP Third Person Character`)))
    (set `self.Active` false :!label _label)
    (`KismetSystemLibrary.K2_ClearTimer` null "TriggerHeartbeat")
    (`Widget.RemoveFromParent` (`self.HeartbeatQTEWidget`))
    (elif (>= (`self.FailCount`) (`self.FailGoal`))
      (bind _outactor (`LevelSequencePlayer.CreateLevelSequencePlayer` (`self.Level Sequence`)))
      (`MovieSceneSequencePlayer.Play` (`LevelSequenceActor.SequencePlayer` _outactor))
      (goto _label))))

(event `self.ReceiveBeginPlay`
  (bind _asbp_third_person_character (cast `/Game/Dynamic/ThirdPerson/Blueprints/BP_ThirdPersonCharacter` (`GameplayStatics.GetPlayerCharacter` 0)))
  (set `self.As BP Third Person Character` _asbp_third_person_character))

(event `self.ReceiveTick`
  (params (DeltaSeconds :type "Float (single-precision)"))
  (bind _heartbeatqtewidget (`self.HeartbeatQTEWidget`))
  (if (`self.Active`)
    (if (`PlayerController.WasInputKeyJustPressed` (`GameplayStatics.GetPlayerController` 0) (`self.InputKey`))
      (set `self.IsKeyPressed` true)
      (if (< (`KismetMathLibrary.Abs` (- (`KismetSystemLibrary.GetGameTimeInSeconds`) (`self.TargetPressTime`))) (`self.InputWindow`))
        (`/Engine/EditorBlueprintResources/StandardMacros.IncrementInt` (`self.SuccessCount`)
          (:`  `
            (`/Game/Dynamic/Systems/QTE/HeartbeatQTE/WB_HeartbeatQTE.PlaySucces` _heartbeatqtewidget)))
        (else
          (`/Engine/EditorBlueprintResources/StandardMacros.IncrementInt` (`self.FailCount`)
            (:`  `
              (`/Game/Dynamic/Systems/QTE/HeartbeatQTE/WB_HeartbeatQTE.PlayFail` _heartbeatqtewidget)))))
      (`self.Outcome`))))

(event `StartQTE`
  (set `self.Active` true)
  (set `self.SuccessCount` 0)
  (set `self.FailCount` 0)
  (set `self.TargetPressTime` 0.0)
  (bind _returnvalue (`|CreateWidget` "/Game/Dynamic/Systems/QTE/HeartbeatQTE/WB_HeartbeatQTE.WB_HeartbeatQTE_C"))
  (bind _output_get (set `self.HeartbeatQTEWidget` _returnvalue))
  (`UserWidget.AddToViewport` _output_get 0)
  (`WidgetBlueprintLibrary.SetInputMode_GameAndUIEx` (`GameplayStatics.GetPlayerController` 0) _output_get)
  (set `self.IsKeyPressed` false))

(event `TriggerHeartbeat`
  (set `self.InputWindow` (`KismetArrayLibrary.Array_Random` (`self.PossibleInputWindows`)))
  (set `self.TargetPressTime` (+ (`KismetSystemLibrary.GetGameTimeInSeconds`) (/ (`self.InputWindow`) 2.0)))
  (set `self.IsKeyPressed` false)
  (bind _output_get (set `self.InputKey` (`KismetArrayLibrary.Array_Random` (`self.PossibleInputKeys`))))
  (`TextBlock.SetText` (`/Game/Dynamic/Systems/QTE/HeartbeatQTE/WB_HeartbeatQTE.InputText` (`self.HeartbeatQTEWidget`)) (`KismetInputLibrary.Key_GetDisplayName` _output_get)))