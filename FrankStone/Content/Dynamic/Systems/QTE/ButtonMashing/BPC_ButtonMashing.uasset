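; Actor component that runs a button-mashing quick time event, where the player must press a key a target number of times before time runs out.
; StartQTE shows the mashing widget, resets state and starts a looping timer, while Tick counts presses of the input key.
; UpdateQTE checks count and elapsed time, sets Success when met, shows SUCCESS or FAIL, then removes the widget and restores game-only input.
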(event `self.ReceiveBeginPlay`)

(event `self.ReceiveTick`
  (params (DeltaSeconds :type "Float (single-precision)"))
  (if (and (`self.Active`) (`PlayerController.WasInputKeyJustPressed` (`GameplayStatics.GetPlayerController` 0) (`self.InputKey`)))
    (`/Engine/EditorBlueprintResources/StandardMacros.IncrementInt` (`self.MashCount`))))

(event `StartQTE`
  (bind _returnvalue (`|CreateWidget` "/Game/Dynamic/Systems/QTE/ButtonMashing/WB_ButtonMashing.WB_ButtonMashing_C" (`GameplayStatics.GetPlayerController` 0)))
  (bind _output_get (set `self.ButtonMashingWidget` _returnvalue))
  (`UserWidget.AddToViewport` _output_get 0)
  (set `self.MashCount` 0)
  (set `self.CurrentTime` 0.0)
  (set `self.Success` false)
  (set `self.Active` true)
  (`KismetSystemLibrary.K2_SetTimer` null "UpdateQTE" 0.1 true)
  (`WidgetBlueprintLibrary.SetInputMode_GameAndUIEx` (`GameplayStatics.GetPlayerController` 0) (`self.ButtonMashingWidget`)))

(event `UpdateQTE`
  (if (not (>= (`self.CurrentTime`) (`self.Duration`)))
    (set `self.CurrentTime` (+ (`self.CurrentTime`) 0.1))
    (if (>= (`self.MashCount`) (`self.TargetMashCount`))
      (set `self.Success` true)
      (`KismetSystemLibrary.K2_ClearTimer` null "UpdateQTE")
      (set `self.Active` false)
      (`Widget.SetVisibility` (`/Game/Dynamic/Systems/QTE/ButtonMashing/WB_ButtonMashing.OutcomeText` (`self.ButtonMashingWidget`)) "Visible")
      (`TextBlock.SetText` (`/Game/Dynamic/Systems/QTE/ButtonMashing/WB_ButtonMashing.OutcomeText` (`self.ButtonMashingWidget`)) "SUCCESS")
      (`Widget.SetVisibility` (`/Game/Dynamic/Systems/QTE/ButtonMashing/WB_ButtonMashing.ButtonText` (`self.ButtonMashingWidget`)) "Hidden")
      (`KismetSystemLibrary.Delay` 1.0)
      (`Widget.RemoveFromParent` (`self.ButtonMashingWidget`))
      (`WidgetBlueprintLibrary.SetInputMode_GameOnly` (`GameplayStatics.GetPlayerController` 0)))
    (else
      (`KismetSystemLibrary.K2_ClearTimer` null "UpdateQTE")
      (set `self.Active` false)
      (`Widget.SetVisibility` (`/Game/Dynamic/Systems/QTE/ButtonMashing/WB_ButtonMashing.OutcomeText` (`self.ButtonMashingWidget`)) "Visible")
      (`TextBlock.SetText` (`/Game/Dynamic/Systems/QTE/ButtonMashing/WB_ButtonMashing.OutcomeText` (`self.ButtonMashingWidget`)) "FAIL")
      (`Widget.SetVisibility` (`/Game/Dynamic/Systems/QTE/ButtonMashing/WB_ButtonMashing.ButtonText` (`self.ButtonMashingWidget`)) "Hidden")
      (`KismetSystemLibrary.Delay` 1.0)
      (`Widget.RemoveFromParent` (`self.ButtonMashingWidget`))
      (`WidgetBlueprintLibrary.SetInputMode_GameOnly` (`GameplayStatics.GetPlayerController` 0)))))