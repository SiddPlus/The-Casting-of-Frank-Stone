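; Actor component that runs timed two-choice dialogue prompts as a QTE through a WB_Choice widget.
; Tick copies the Dialogue entry at DialogueIndex into the button texts, outcomes and next indices.
; StartQTE shows the widget and cursor, binds both buttons and starts a looping countdown that defaults to choice A on timeout.
; Choosing prints the outcome, advances DialogueIndex along that branch, then hides the widget and restores game input.
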(event `self.ReceiveBeginPlay`
  (bind _returnvalue (`|CreateWidget` "/Game/Dynamic/Systems/QTE/Dialogue/WB_Choice.WB_Choice_C" (`GameplayStatics.GetPlayerController` 0)))
  (bind _output_get (set `self.ChoiceWidget` _returnvalue))
  (`UserWidget.AddToViewport` _output_get 0)
  (`Widget.SetVisibility` (`self.ChoiceWidget`) "Hidden"))

(event `self.ReceiveTick`
  (params (DeltaSeconds :type "Float (single-precision)"))
  (bind _choicewidget (`self.ChoiceWidget`))
  (for (_array_element _array_index) (`self.Dialogue`)
    (if (== _array_index (`self.DialogueIndex`))
      (bind (_question _choicea _choiceb _outcomea _outcomeb _nextdialogueindexa _nextdialogueindexb) (break `/Game/Dynamic/Systems/QTE/Dialogue/S_Dialogue` _array_element))
      (set `TextBlock.Text` _choicea (`/Game/Dynamic/Systems/QTE/Dialogue/WB_Choice.TextChoiceA` _choicewidget))
      (set `TextBlock.Text` _choiceb (`/Game/Dynamic/Systems/QTE/Dialogue/WB_Choice.TextChiceB` _choicewidget))
      (set `self.Outcome A` _outcomea)
      (set `self.Outcome B` _outcomeb)
      (set `self.Next Dialogue Index A` _nextdialogueindexa)
      (set `self.Next Dialogue Index B` _nextdialogueindexb))))

(event `Start QTE`
  (bind _returnvalue (`GameplayStatics.GetPlayerController` 0))
  (bind _choicewidget (`self.ChoiceWidget`))
  (`Widget.SetVisibility` (`self.ChoiceWidget`) "Visible")
  (set `PlayerController.bShowMouseCursor` true _returnvalue)
  (`WidgetBlueprintLibrary.SetInputMode_GameAndUIEx` _returnvalue null)
  (`KismetSystemLibrary.K2_SetTimer` null "Update QTE" 1.0 true)
  (add `Button.OnClicked` (`/Game/Dynamic/Systems/QTE/Dialogue/WB_Choice.Button_A` _choicewidget) (delegate `Handle QTE Choice A`))
  (add `Button.OnClicked` (`/Game/Dynamic/Systems/QTE/Dialogue/WB_Choice.Button_B` _choicewidget) (delegate `Handle QTE Choice B`)))

(event `Handle QTE Choice B`
  (bind _returnvalue (`GameplayStatics.GetPlayerController` 0))
  (set `self.Selection` "NewEnumerator2")
  (switch `/Game/Dynamic/Systems/QTE/Dialogue/E_Choice` (`self.Selection`) :!label _label
    (:`NewEnumerator1`
      (`KismetSystemLibrary.PrintString` (`self.Outcome A`))
      (set `self.DialogueIndex` (`self.Next Dialogue Index A`)))
    (:`NewEnumerator2`
      (`KismetSystemLibrary.PrintString` (`self.Outcome B`))
      (set `self.DialogueIndex` (`self.Next Dialogue Index B`))))
  (set `PlayerController.bShowMouseCursor` false _returnvalue)
  (`WidgetBlueprintLibrary.SetInputMode_GameOnly` _returnvalue)
  (`Widget.SetVisibility` (`self.ChoiceWidget`) "Hidden")
  (`KismetSystemLibrary.K2_ClearTimer` null "Update QTE")
  (set `self.TimeRemaining` 5.0))

(event `Handle QTE Choice A`
  (set `self.Selection` "NewEnumerator1")
  (goto _label))

(event `Update QTE`
  (`/Engine/EditorBlueprintResources/StandardMacros.DecrementFloat` (`self.TimeRemaining`)
    (:`  `
      (if (<= (`self.TimeRemaining`) 0.0)
        (`self.Handle QTE Choice A`)
        (set `self.TimeRemaining` 5.0)))))