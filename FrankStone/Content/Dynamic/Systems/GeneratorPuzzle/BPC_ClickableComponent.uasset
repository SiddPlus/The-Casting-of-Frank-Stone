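; Clickable component for generator puzzle buttons that adds hover outlines and records clicks into the player's button sequence.
; On BeginPlay it binds owner cursor events, toggles the mesh's custom depth on hover, and caches the character and owning BP_Button.
; Clicks push the button, then branch on length and match checks to activate the puzzle or reset it.
; Both check functions contain button-versus-lever sequence comparisons that are left unconnected.
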(event `self.ReceiveBeginPlay`
  (bind _returnvalue (`self.GetOwner`))
  (bind _returnvalue_2 (`Actor.GetComponentByClass` _returnvalue "/Script/Engine.StaticMeshComponent"))
  (add `Actor.OnClicked` _returnvalue (delegate `OnMouseClicked`))
  ;[1 1 1] Get owners static mesh if owner has one
  (`/Engine/EditorBlueprintResources/StandardMacros.IsValid` _returnvalue_2
    (:`Is Valid`
      (set `self.Static Mesh Ref` _returnvalue_2)
      (add `Actor.OnBeginCursorOver` _returnvalue (delegate `OnMouseHover`))
      (add `Actor.OnEndCursorOver` _returnvalue (delegate `OnMouseHoverEnd`))
      (bind _asbp_third_person_character (cast `/Game/Dynamic/ThirdPerson/Blueprints/BP_ThirdPersonCharacter` (`GameplayStatics.GetPlayerCharacter` 0)))
      (set `self.As BP Third Person Character` _asbp_third_person_character)
      (bind _asbp_button (cast `/Game/Dynamic/Systems/GeneratorPuzzle/BP_Button` (`self.GetOwner`)))
      (set `self.As BP Button` _asbp_button))))

(event `OnMouseHover`
  (params (TouchedActor :type "Actor Object Reference"))
  ;[1 1 1] Create Outline of static mesh on Mouse hover
  (`PrimitiveComponent.SetRenderCustomDepth` (`self.Static Mesh Ref`) true))

(event `OnMouseHoverEnd`
  (params (TouchedActor :type "Actor Object Reference"))
  ;[1 1 1] Create Outline of static mesh on Mouse hover
  (`PrimitiveComponent.SetRenderCustomDepth` (`self.Static Mesh Ref`) false))

(event `OnMouseClicked`
  (params (TouchedActor :type "Actor Object Reference") (ButtonPressed :type "Key Structure" :default "None"))
  (bind _as_bp_button (`self.As BP Button`))
  (bind _bpc_correctsequence (`/Game/Dynamic/ThirdPerson/Blueprints/BP_ThirdPersonCharacter.BPC_CorrectSequence` (`self.As BP Third Person Character`)))
  (bind _bpc_correctsequence_2 (`/Game/Dynamic/ThirdPerson/Blueprints/BP_ThirdPersonCharacter.BPC_CorrectSequence` (`self.As BP Third Person Character`)))
  (if (not (`/Game/Dynamic/Systems/GeneratorPuzzle/BP_Button.IsPushed` _as_bp_button))
    (set `/Game/Dynamic/Systems/GeneratorPuzzle/BP_Button.IsPushed` true _as_bp_button)
    (`/Game/Dynamic/Systems/GeneratorPuzzle/BPC_CorrectSequence.Add to UI Button Sequence` (`/Game/Dynamic/ThirdPerson/Blueprints/BP_ThirdPersonCharacter.BPC_CorrectSequence` (`self.As BP Third Person Character`)) (`/Game/Dynamic/Systems/GeneratorPuzzle/BP_Button.ID` (`self.As BP Button`)) (`self.As BP Button`))
    (if (== (`KismetArrayLibrary.Array_Length` (`/Game/Dynamic/Systems/GeneratorPuzzle/BPC_CorrectSequence.PlayerButtonSequence` _bpc_correctsequence)) (`KismetArrayLibrary.Array_Length` (`/Game/Dynamic/Systems/GeneratorPuzzle/BPC_CorrectSequence.PlayerLeverSequence` _bpc_correctsequence)))
      (if (`KismetArrayLibrary.Array_Identical` (`/Game/Dynamic/Systems/GeneratorPuzzle/BPC_CorrectSequence.PlayerButtonSequence` _bpc_correctsequence_2) (`/Game/Dynamic/Systems/GeneratorPuzzle/BPC_CorrectSequence.PlayerLeverSequence` _bpc_correctsequence_2))
        (set `/Game/Dynamic/Systems/GeneratorPuzzle/BPC_CorrectSequence.IsActivated` true (`/Game/Dynamic/ThirdPerson/Blueprints/BP_ThirdPersonCharacter.BPC_CorrectSequence` (`self.As BP Third Person Character`)))
        (`/Game/Dynamic/Systems/GeneratorPuzzle/BPC_CorrectSequence.Remove Widget` (`/Game/Dynamic/ThirdPerson/Blueprints/BP_ThirdPersonCharacter.BPC_CorrectSequence` (`self.As BP Third Person Character`)))
        (`KismetSystemLibrary.PrintString` "Activated")
        (else
          (`KismetArrayLibrary.Array_Clear` (`/Game/Dynamic/Systems/GeneratorPuzzle/BPC_CorrectSequence.PlayerButtonSequence` (`/Game/Dynamic/ThirdPerson/Blueprints/BP_ThirdPersonCharacter.BPC_CorrectSequence` (`self.As BP Third Person Character`))))
          (for _array_element (`/Game/Dynamic/Systems/GeneratorPuzzle/BPC_CorrectSequence.BP_Button` (`/Game/Dynamic/ThirdPerson/Blueprints/BP_ThirdPersonCharacter.BPC_CorrectSequence` (`self.As BP Third Person Character`)))
            (set `/Game/Dynamic/Systems/GeneratorPuzzle/BP_Button.IsPushed` false _array_element)
            (`KismetSystemLibrary.PrintString` "Failed to activate")))))))