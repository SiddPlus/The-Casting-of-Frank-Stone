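; Base interactable actor in the generator puzzle system, identified by an ID and shown with a configurable mesh assigned at BeginPlay.
; It caches the player character, and Interact switches off that character's BPCFlash aiming, prints a debug message and returns its ID and itself as LeverButton.
; Any end overlap on its sphere switches aiming back on, with no check on which actor left.
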(event `self.ReceiveBeginPlay`
  (`StaticMeshComponent.SetStaticMesh` (`self.StaticMesh`) (`self.Mesh`))
  (bind _asbp_third_person_character (cast `/Game/Dynamic/ThirdPerson/Blueprints/BP_ThirdPersonCharacter` (`GameplayStatics.GetPlayerCharacter` 0)))
  (set `self.As BP Third Person Character` _asbp_third_person_character))

(event `self.ReceiveTick`
  (params (DeltaSeconds :type "Float (single-precision)")))

(event `self.Sphere.OnComponentEndOverlap`
  (params (OverlappedComponent :type "PrimitiveComponent Object Reference") (OtherActor :type "Actor Object Reference") (OtherComp :type "PrimitiveComponent Object Reference") (OtherBodyIndex :type Integer))
  (bind _bpc_flash (`/Game/Dynamic/ThirdPerson/Blueprints/BP_ThirdPersonCharacter.BPC_Flash` (`self.As BP Third Person Character`)))
  (bind _output_get (set `/Game/Dynamic/Systems/Flash/BPC_Flash.IsAiming` true _bpc_flash))
  (`/Game/Dynamic/Systems/Flash/BPC_Flash.ToggleAiming` _bpc_flash _output_get))

(fn `Interact`
  (returns (ID :type Integer) (`Lever/Button` :type "/Game/Dynamic/Systems/GeneratorPuzzle/BP_Interactable Object Reference"))
  (bind _bpc_flash (`/Game/Dynamic/ThirdPerson/Blueprints/BP_ThirdPersonCharacter.BPC_Flash` (`self.As BP Third Person Character`)))
  (bind _output_get (set `/Game/Dynamic/Systems/Flash/BPC_Flash.IsAiming` false _bpc_flash))
  (`/Game/Dynamic/Systems/Flash/BPC_Flash.ToggleAiming` _bpc_flash _output_get)
  (`KismetSystemLibrary.PrintString` "ON")
  (return (`self.ID`) self))

(fn `UserConstructionScript`)