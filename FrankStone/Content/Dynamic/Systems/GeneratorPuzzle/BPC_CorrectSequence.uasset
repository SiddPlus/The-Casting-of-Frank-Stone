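; Component for the generator puzzle that records the player's lever and button sequences and controls the generator UI.
; It creates a hidden WB_Generator widget on BeginPlay, then shows or hides it through events that switch cursor, input mode and the SwapToGen flag, with a short delay before showing.
; Add functions store each pressed ID alongside its lever, button or UI button, with both button types sharing one ID sequence.
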(event `self.ReceiveBeginPlay`
  (bind _returnvalue (`|CreateWidget` "/Game/Dynamic/Systems/GeneratorPuzzle/WB_Generator.WB_Generator_C" (`GameplayStatics.GetPlayerController` 0)))
  (bind _output_get (set `self.GeneratorWidget` _returnvalue))
  (`UserWidget.AddToViewport` _output_get 0)
  (`Widget.SetVisibility` (`self.GeneratorWidget`) "Hidden"))

(event `CreateWidget`
  (bind _returnvalue (`GameplayStatics.GetPlayerController` 0))
  (set `self.SwapToGen` true)
  (`KismetSystemLibrary.Delay` 0.5)
  (`Widget.SetVisibility` (`self.GeneratorWidget`) "Visible")
  (set `PlayerController.bShowMouseCursor` true _returnvalue)
  (`WidgetBlueprintLibrary.SetInputMode_GameAndUIEx` _returnvalue (`self.GeneratorWidget`)))

(event `Remove Widget`
  (bind _returnvalue (`GameplayStatics.GetPlayerController` 0))
  (`Widget.SetVisibility` (`self.GeneratorWidget`) "Hidden")
  (set `PlayerController.bShowMouseCursor` false _returnvalue)
  (`WidgetBlueprintLibrary.SetInputMode_GameOnly` _returnvalue)
  (set `self.SwapToGen` false))

(fn `Add To Button Sequence`
  (params (ID :type Integer) (Button :type "/Game/Dynamic/Systems/GeneratorPuzzle/BP_Interactable Object Reference"))
  (`KismetArrayLibrary.Array_Add` (`self.PlayerButtonSequence`) ID)
  (`KismetArrayLibrary.Array_Add` (`self.Buttons`) Button))

(fn `Add To Lever Sequence`
  (params (ID :type Integer) (Lever :type "/Game/Dynamic/Systems/GeneratorPuzzle/BP_Interactable Object Reference"))
  (`KismetArrayLibrary.Array_Add` (`self.PlayerLeverSequence`) ID)
  (`KismetArrayLibrary.Array_Add` (`self.Levers`) Lever))

(fn `Add to UI Button Sequence`
  (params (ID :type Integer) (UIButton :type "/Game/Dynamic/Systems/GeneratorPuzzle/BP_Button Object Reference"))
  (`KismetArrayLibrary.Array_Add` (`self.PlayerButtonSequence`) ID)
  (`KismetArrayLibrary.Array_Add` (`self.BP_Button`) UIButton))