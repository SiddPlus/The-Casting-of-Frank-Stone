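; Player camera-mode component that switches the third-person character into an aimed camera view and fires a spotlight flash.
; ToggleAiming sets FOV and camera offset targets, hides the mesh, deactivates movement and shows the WB_Camera widget, reversing this on exit.
; Tick eases the follow camera toward those targets and fades the spotlight.
; TriggerFlash raises the light intensity and clears CanFlash, which Tick restores once intensity reaches zero.
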(event `self.ReceiveBeginPlay`
  (bind _asbp_third_person_character (cast `/Game/Dynamic/ThirdPerson/Blueprints/BP_ThirdPersonCharacter` (`GameplayStatics.GetPlayerCharacter` 0)))
  (set `self.As BP Third Person Character` _asbp_third_person_character)
  (set `self.TargetFoV` (`self.DefaultFOV`)))

(event `self.ReceiveTick`
  (params (DeltaSeconds :type "Float (single-precision)"))
  (bind _relativelocation_x (`KismetMathLibrary.BreakVector` (`SceneComponent.RelativeLocation` (`/Game/Dynamic/ThirdPerson/Blueprints/BP_ThirdPersonCharacter.FollowCamera` (`self.As BP Third Person Character`)))))
  (bind (_relativelocation_x_2 _relativelocation_y _relativelocation_z) (`KismetMathLibrary.BreakVector` (`SceneComponent.RelativeLocation` (`/Game/Dynamic/ThirdPerson/Blueprints/BP_ThirdPersonCharacter.FollowCamera` (`self.As BP Third Person Character`)))))
  (set `self.Delta Seconds` DeltaSeconds)
  (`SceneComponent.K2_SetRelativeTransform` (`/Game/Dynamic/ThirdPerson/Blueprints/BP_ThirdPersonCharacter.FollowCamera` (`self.As BP Third Person Character`)) (`KismetMathLibrary.MakeTransform` (`KismetMathLibrary.MakeVector` (`KismetMathLibrary.FInterpTo` _relativelocation_x (`self.XTarget`) (`self.Delta Seconds`) (`self.AimSpeed`)) 0.0 (`KismetMathLibrary.FInterpTo` _relativelocation_z (`self.ZTarget`) (`self.Delta Seconds`) (`self.AimSpeed`)))) false false)
  (set `CameraComponent.FieldOfView` (`KismetMathLibrary.FInterpTo` (`CameraComponent.FieldOfView` (`/Game/Dynamic/ThirdPerson/Blueprints/BP_ThirdPersonCharacter.FollowCamera` (`self.As BP Third Person Character`))) (`self.TargetFoV`) (`self.Delta Seconds`) (`self.AimSpeed`)) (`/Game/Dynamic/ThirdPerson/Blueprints/BP_ThirdPersonCharacter.FollowCamera` (`self.As BP Third Person Character`)))
  (`LightComponent.SetIntensity` (`/Game/Dynamic/ThirdPerson/Blueprints/BP_ThirdPersonCharacter.SpotLight` (`self.As BP Third Person Character`)) (`KismetMathLibrary.FInterpTo` (`LightComponentBase.Intensity` (`/Game/Dynamic/ThirdPerson/Blueprints/BP_ThirdPersonCharacter.SpotLight` (`self.As BP Third Person Character`))) 0.0 (`self.Delta Seconds`) (`self.DimSpeed`)))
  (if (== (`LightComponentBase.Intensity` (`/Game/Dynamic/ThirdPerson/Blueprints/BP_ThirdPersonCharacter.SpotLight` (`self.As BP Third Person Character`))) 0.0)
    (set `self.CanFlash` true)))

(fn `ToggleAiming`
  (params (NewState :type Boolean))
  (set `self.IsAiming` NewState)
  (if (`self.IsAiming`)
    (set `self.TargetFoV` (`self.AimFOV`))
    (set `self.XTarget` (`self.XAim`))
    (set `self.ZTarget` (`self.ZAim`))
    (set `self.IsInCameraMode` true)
    (`SceneComponent.SetVisibility` (`Character.Mesh` (`self.As BP Third Person Character`)) false false)
    (bind _returnvalue (`|CreateWidget` "/Game/Dynamic/Systems/Flash/WB_Camera.WB_Camera_C" (`GameplayStatics.GetPlayerController` 0)))
    (bind _output_get (set `self.CameraWidget` _returnvalue))
    (`UserWidget.AddToViewport` _output_get 0)
    (`self.Deactivate` (`Character.CharacterMovement` (`self.As BP Third Person Character`)))
    (else
      (set `self.TargetFoV` (`self.DefaultFOV`))
      (set `self.XTarget` (`self.DefaultX`))
      (set `self.ZTarget` (`self.DefaultZ`))
      (set `self.IsInCameraMode` false)
      (`SceneComponent.SetVisibility` (`Character.Mesh` (`self.As BP Third Person Character`)) true false)
      (`Widget.RemoveFromParent` (`self.CameraWidget`))
      (`self.Activate` (`Character.CharacterMovement` (`self.As BP Third Person Character`)) false))))

(fn `TriggerFlash`
  (`LightComponent.SetIntensity` (`/Game/Dynamic/ThirdPerson/Blueprints/BP_ThirdPersonCharacter.SpotLight` (`self.As BP Third Person Character`)) (`self.New Intensity`))
  (set `self.CanFlash` false))